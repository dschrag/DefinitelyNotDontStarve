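; BP_ScaryThing is a cave-generation actor that creeps toward the player when it can see them.
; Each tick while overlapping the player pawn, it fires a debug-drawn visibility trace toward them and prints the hit actor's name.
; If that name matches the player's, it teleports one unit along that direction, so movement speed depends on frame rate.
; The construction script scales Sphere1 by CollisionSphereScale.
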(event EventBeginPlay)

(event Collision|EventActorBeginOverlap
  (params (OtherActor :type Actor%20Object%20Reference)))

(event EventTick
  (params (DeltaSeconds :type Float%20%28single-precision%29))
  (bind _returnvalue (Transformation|GetActorLocation))
  (bind _returnvalue_2 (Game|Player|GetPlayerPawn 0))
  (bind _returnvalue_3 (Transformation|GetActorLocation))
  (if (Collision|IsOverlappingActor self _returnvalue_2 :!class /Script/Engine.Actor)
    (bind (_outhit _returnvalue_4) (Collision|LineTraceByChannel _returnvalue_3 (+ (* (Class|KismetMathLibrary|GetDirectionVector _returnvalue_3 (Transformation|GetActorLocation _returnvalue_2)) 1e+03) _returnvalue_3) "TraceTypeQuery1" false 0 "ForOneFrame"))
    (if _returnvalue_4
      (Development|PrintString (Utilities|GetDisplayName (.HitActor (Collision|BreakHitResult _outhit))))
      (if (Utilities|Enum|Equal(Enum) (Utilities|GetDisplayName (.HitActor (Collision|BreakHitResult _outhit))) (Utilities|GetDisplayName (Game|Player|GetPlayerPawn 0)))
        (Transformation|Teleport (+ (Class|KismetMathLibrary|GetDirectionVector _returnvalue (Transformation|GetActorLocation (Game|Player|GetPlayerPawn 0))) _returnvalue) "0, 0, 0")))))

(fn ConstructionScript
  (bind _collision_sphere_scale (Variables|Default|GetCollision%20Sphere%20Scale))
  (Transformation|SetRelativeTransform (Variables|Default|GetSphere1) (Math|Transform|MakeTransform "0, 0, 0" "0, 0, 0" (Math|Vector|MakeVector _collision_sphere_scale _collision_sphere_scale _collision_sphere_scale)) false false))