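; BP_Sign is a sign actor in the CaveGeneration folder that displays up to four lines of text.
; Its construction script converts the Line1 to Line4 variables to text and writes each to its own text render component.
; The event graph holds only disabled placeholder events, so the sign has no runtime logic.
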(event EventBeginPlay)

(event Collision|EventActorBeginOverlap
  (params (OtherActor :type Actor%20Object%20Reference)))

(event EventTick
  (params (DeltaSeconds :type Float%20%28single-precision%29)))

(fn ConstructionScript
  (Rendering|Components|TextRender|SetText (Variables|Default|GetText) (Utilities|Text|ToText(String) (Variables|Default|GetLine1)))
  (Rendering|Components|TextRender|SetText (Variables|Default|GetTextRender) (Utilities|Text|ToText(String) (Variables|Default|GetLine2)))
  (Rendering|Components|TextRender|SetText (Variables|Default|GetTextRender1) (Utilities|Text|ToText(String) (Variables|Default|GetLine3)))
  (Rendering|Components|TextRender|SetText (Variables|Default|GetTextRender2) (Utilities|Text|ToText(String) (Variables|Default|GetLine4))))