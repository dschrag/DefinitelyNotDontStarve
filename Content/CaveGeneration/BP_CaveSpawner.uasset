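; Cave generation spawner that chooses a tile's open door directions and spawns a random matching cave segment at its transform.
; The construction script keeps required directions, excludes restricted ones and opens each other one at one-in-three odds, despite a 1/4 comment.
; On spawn request, door count and layout select the I, L, T, X or dead-end pool.
; The spawned cave receives the directions and counts its item spawns.
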(event Custom|On%20Spawn%20Requested
  (Variables|Default|SetDoors%20That%20Are%20Open (Variables|Default|GetActual%20Spawn%20Doors))
  (if (Math|Boolean|ANDBoolean (Utilities|Array|ContainsItem (Variables|Default|GetDoors%20That%20Are%20Open) "NewEnumerator2") (Utilities|Array|ContainsItem (Variables|Default|GetDoors%20That%20Are%20Open) "NewEnumerator3") (== (Utilities|Array|Length (Variables|Default|GetDoors%20That%20Are%20Open)) 2)) ; Horizontal
    (CallFunction|SpawnRandomCavefrom (Variables|Default|GetI%20Caves) :!label _label)
    (elif (Math|Boolean|ANDBoolean (Utilities|Array|ContainsItem (Variables|Default|GetDoors%20That%20Are%20Open) "NewEnumerator0") (Utilities|Array|ContainsItem (Variables|Default|GetDoors%20That%20Are%20Open) "NewEnumerator1") (== (Utilities|Array|Length (Variables|Default|GetDoors%20That%20Are%20Open)) 2)) ; Vertical
      (goto _label)
      (elif (Math|Boolean|ANDBoolean (Utilities|Array|ContainsItem (Variables|Default|GetDoors%20That%20Are%20Open) "NewEnumerator2") (Utilities|Array|ContainsItem (Variables|Default|GetDoors%20That%20Are%20Open) "NewEnumerator3") (Utilities|Array|ContainsItem (Variables|Default|GetDoors%20That%20Are%20Open) "NewEnumerator0") (Utilities|Array|ContainsItem (Variables|Default|GetDoors%20That%20Are%20Open) "NewEnumerator1"))
        (CallFunction|SpawnRandomCavefrom (Variables|Default|GetX%20Caves))
        (elif (Math|Boolean|ANDBoolean (Utilities|Array|ContainsItem (Variables|Default|GetDoors%20That%20Are%20Open) "NewEnumerator0") (Utilities|Array|ContainsItem (Variables|Default|GetDoors%20That%20Are%20Open) "NewEnumerator2") (== (Utilities|Array|Length (Variables|Default|GetDoors%20That%20Are%20Open)) 2)) ; L
          (CallFunction|SpawnRandomCavefrom (Variables|Default|GetL%20Caves) :!label _label_2)
          (elif (Math|Boolean|ANDBoolean (Utilities|Array|ContainsItem (Variables|Default|GetDoors%20That%20Are%20Open) "NewEnumerator2") (Utilities|Array|ContainsItem (Variables|Default|GetDoors%20That%20Are%20Open) "NewEnumerator1") (== (Utilities|Array|Length (Variables|Default|GetDoors%20That%20Are%20Open)) 2)) ; L
            (goto _label_2)
            (elif (Math|Boolean|ANDBoolean (Utilities|Array|ContainsItem (Variables|Default|GetDoors%20That%20Are%20Open) "NewEnumerator1") (Utilities|Array|ContainsItem (Variables|Default|GetDoors%20That%20Are%20Open) "NewEnumerator3") (== (Utilities|Array|Length (Variables|Default|GetDoors%20That%20Are%20Open)) 2)) ; L
              (goto _label_2)
              (elif (Math|Boolean|ANDBoolean (Utilities|Array|ContainsItem (Variables|Default|GetDoors%20That%20Are%20Open) "NewEnumerator3") (Utilities|Array|ContainsItem (Variables|Default|GetDoors%20That%20Are%20Open) "NewEnumerator0") (== (Utilities|Array|Length (Variables|Default|GetDoors%20That%20Are%20Open)) 2)) ; L
                (goto _label_2)
                (elif (and (not (Utilities|Array|ContainsItem (Variables|Default|GetDoors%20That%20Are%20Open) "NewEnumerator3")) (== (Utilities|Array|Length (Variables|Default|GetDoors%20That%20Are%20Open)) 3)) ; T
                  (CallFunction|SpawnRandomCavefrom (Variables|Default|GetT%20Caves) :!label _label_3)
                  (elif (and (not (Utilities|Array|ContainsItem (Variables|Default|GetDoors%20That%20Are%20Open) "NewEnumerator0")) (== (Utilities|Array|Length (Variables|Default|GetDoors%20That%20Are%20Open)) 3)) ; T
                    (goto _label_3)
                    (elif (and (not (Utilities|Array|ContainsItem (Variables|Default|GetDoors%20That%20Are%20Open) "NewEnumerator2")) (== (Utilities|Array|Length (Variables|Default|GetDoors%20That%20Are%20Open)) 3)) ; T
                      (goto _label_3)
                      (elif (and (not (Utilities|Array|ContainsItem (Variables|Default|GetDoors%20That%20Are%20Open) "NewEnumerator1")) (== (Utilities|Array|Length (Variables|Default|GetDoors%20That%20Are%20Open)) 3)) ; T
                        (goto _label_3)
                        (elif (and (Utilities|Array|ContainsItem (Variables|Default|GetDoors%20That%20Are%20Open) "NewEnumerator3") (== (Utilities|Array|Length (Variables|Default|GetDoors%20That%20Are%20Open)) 1)) ; Dead End
                          (CallFunction|SpawnRandomCavefrom (Variables|Default|GetDead%20End%20Caves) :!label _label_4)
                          (elif (and (Utilities|Array|ContainsItem (Variables|Default|GetDoors%20That%20Are%20Open) "NewEnumerator0") (== (Utilities|Array|Length (Variables|Default|GetDoors%20That%20Are%20Open)) 1)) ; Dead End
                            (goto _label_4)
                            (elif (and (Utilities|Array|ContainsItem (Variables|Default|GetDoors%20That%20Are%20Open) "NewEnumerator2") (== (Utilities|Array|Length (Variables|Default|GetDoors%20That%20Are%20Open)) 1)) ; Dead End
                              (goto _label_4)
                              (elif (and (Utilities|Array|ContainsItem (Variables|Default|GetDoors%20That%20Are%20Open) "NewEnumerator1") (== (Utilities|Array|Length (Variables|Default|GetDoors%20That%20Are%20Open)) 1)) ; Dead end
                                (goto _label_4)))))))))))))))))

(event Custom|On%20Do%20Door%20Choice
  (bind _door_directions (CallFunction|OpenMoreDoors (Variables|Default|GetMinimum%20Door%20Directions) (Variables|Default|GetRestricted%20Door%20Directions)))
  (Variables|Default|SetActual%20Spawn%20Doors _door_directions))

(event EventBeginPlay)

(event Collision|EventActorBeginOverlap
  (params (OtherActor :type Actor%20Object%20Reference)))

(event EventTick
  (params (DeltaSeconds :type Float%20%28single-precision%29)))

(fn ConstructionScript
  (CallFunction|OnDoDoorChoice))

(fn SpawnRandomCavefrom
  (params (Caves :type Array%20of%20BP%20Cave%20Parent%20Class%20References))
  (bind _returnvalue (Game|SpawnActorfromClass (Utilities|Array|Get(acopy) Caves (Math|Random|RandomIntegerinRange 0 (- (Utilities|Array|Length Caves) 1))) (Transformation|GetActorTransform) "Undefined" self (Variables|Default|GetActual%20Spawn%20Doors) 0))
  (bind _output_get (Variables|Default|SetSpawned%20Cave _returnvalue))
  (Default|CountItemSpawns _output_get)
  (return))

(fn OpenMoreDoors
  (params (Required :type Array%20of%20Enum_Directions%20Enums) (Restricted :type Array%20of%20Enum_Directions%20Enums))
  (LocalVariables|SetRequired%20Directions Required)
  (LocalVariables|SetRestricted%20Directions Restricted)
  (bind _enumvalue (|ForEachEnum_Directions)
    (:LoopBody
      (if (Utilities|Array|ContainsItem (LocalVariables|GetRequired%20Directions) _enumvalue) ; Is explicitly required
        (Utilities|Array|Add (LocalVariables|GetOutput%20Directions) _enumvalue)
        (elif (not (Utilities|Array|ContainsItem (LocalVariables|GetRestricted%20Directions) _enumvalue)) ; is explicitly banned
          (if (== (Math|Random|RandomInteger 3) 0) ; Is randomly determined to be open
            (Utilities|Array|Add (LocalVariables|GetOutput%20Directions) _enumvalue)))))
    (:then
      (return (LocalVariables|GetOutput%20Directions)))))