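; BP_Rat is a rat actor for cave generation that makes ambient squeaks and can be killed by an attack.
; Tick calls the parent, then uses a random-length Delay as a throttle to play a quiet, attenuated idle sound every several seconds.
; OnAttacked spawns a BP_RatCarcas at the rat's transform, plays a death sound there and destroys the actor.
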(event EventBeginPlay)

(event Collision|EventActorBeginOverlap
  (params (OtherActor :type Actor%20Object%20Reference)))

(event EventTick
  (params (DeltaSeconds :type Float%20%28single-precision%29))
  (|CallParentFunction 0.0)
  (Utilities|FlowControl|Delay (Math|Conversions|ToFloat(Integer) (Math|Random|RandomIntegerinRange 8 16)))
  (Audio|PlaySoundatLocation "/Game/Audio/ratidlewav.ratidlewav" (Transformation|GetActorLocation) "0, 0, 0" 0.1 1.0 0.0 (Variables|Default|GetAttenuationSettings)))

(event EventOnAttacked
  (bind _returnvalue (Transformation|GetActorTransform))
  (Game|SpawnActorfromClass "/Game/CaveGeneration/Items/BP_RatCarcas.BP_RatCarcas_C" _returnvalue "Undefined" 0 0)
  (Audio|PlaySoundatLocation "/Game/Audio/deathd.deathd" (.Location (Math|Transform|BreakTransform _returnvalue)))
  (Actor|DestroyActor))

(fn ConstructionScript
  (|CallParentFunction))