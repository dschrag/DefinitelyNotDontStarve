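; Scary creature for cave generation that creeps toward the player and is destroyed when attacked.
; Each Tick while overlapping the player pawn, it line-traces toward them and, if they are hit first, teleports one unit closer, so speed is frame-rate dependent.
; It yaws MeshCenter toward the player with an adjustable offset, first snapping it to the floor unless DoesFly.
; The Construction Script scales the collision Sphere from CollisionSphereScale.
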(event Custom|On%20Attacked
  (Development|PrintString "Ouch! You killed a rat!")
  (Actor|DestroyActor))

(event EventBeginPlay)

(event Collision|EventActorBeginOverlap
  (params (OtherActor :type Actor%20Object%20Reference)))

(event EventTick
  (params (DeltaSeconds :type Float%20%28single-precision%29))
  (bind _returnvalue (Transformation|GetActorLocation))
  (bind _returnvalue_2 (Transformation|GetActorLocation))
  (bind _returnvalue_3 (Game|Player|GetPlayerPawn 0))
  (bind _returnvalue_4 (Transformation|GetActorLocation))
  (bind _mesh_center (Variables|Default|GetMesh%20Center))
  (bind _returnvalue_5 (Transformation|GetWorldRotation _mesh_center))
  (if (Collision|IsOverlappingActor _returnvalue_3 :!class /Script/Engine.Actor)
    (bind (_outhit _returnvalue_6) (Collision|LineTraceByChannel _returnvalue_4 (+ (* (Class|KismetMathLibrary|GetDirectionVector _returnvalue_4 (Transformation|GetActorLocation _returnvalue_3)) 1e+03) _returnvalue_4) "TraceTypeQuery1" false 0 "ForOneFrame"))
    (if _returnvalue_6
      (Development|PrintString (Utilities|GetDisplayName (.HitActor (Collision|BreakHitResult _outhit))))
      (if (Utilities|Enum|Equal(Enum) (Utilities|GetDisplayName (.HitActor (Collision|BreakHitResult _outhit))) (Utilities|GetDisplayName (Game|Player|GetPlayerPawn 0)))
        (Transformation|Teleport (+ (Class|KismetMathLibrary|GetDirectionVector _returnvalue (Transformation|GetActorLocation (Game|Player|GetPlayerPawn 0))) _returnvalue) "0, 0, 0")
        (if (Variables|Default|GetDoes%20Fly?)
          _
          (else
            ;[1 1 1] Make it touch the floor.
            (bind _outhit_2 (Collision|LineTraceByChannel (Transformation|GetActorLocation) (Math|Vector|MakeVector (.x _returnvalue_2) (.y _returnvalue_2) -1e+03) "TraceTypeQuery1" false 0 "None"))
            (Transformation|SetWorldLocation (Variables|Default|GetMesh%20Center) (.Location (Collision|BreakHitResult _outhit_2)) false true)))
        ;[1 1 1] Make it face the player
        (Transformation|SetWorldRotation (Variables|Default|GetMesh%20Center) (Math|Rotator|MakeRotator (.roll _returnvalue_5) (.pitch _returnvalue_5) (+ (.yaw (Math|Rotator|FindLookatRotation (Transformation|GetActorLocation) (Transformation|GetActorLocation (Game|Player|GetPlayerPawn 0)))) (Variables|Default|GetLook%20at%20Z%20Adjustment))) false false))
      (else
        (Development|PrintString "Nope, no trace")))))

(fn ConstructionScript
  (bind _collision_sphere_scale (Variables|Default|GetCollision%20Sphere%20Scale))
  (Transformation|SetRelativeTransform (Variables|Default|GetSphere) (Math|Transform|MakeTransform "0, 0, 0" "0, 0, 0" (Math|Vector|MakeVector _collision_sphere_scale _collision_sphere_scale _collision_sphere_scale)) false false))