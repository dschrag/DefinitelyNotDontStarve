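; Item distributor that spawns required and optional items at spawn points received when cave generation finishes.
; CaveGenerated stores the points, then spawns each required item using PopRandomSpawnLocation, which removes the last point and returns the new last one.
; Each remaining point then rolls a weighted chance to spawn the item from GetRandomOptionalItem.
; Despite their names, both helpers index the array end rather than choosing randomly.
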(event Custom|Cave%20Generated
  (params (Available%20Spawns :type Array%20of%20S%20Item%20Spawn%20Point%20Structures))
  (bind _output_get (Variables|Default|SetAvailable%20Spawn%20Points Available%20Spawns))
  (Development|PrintString (Utilities|String|Append "There are " (Utilities|String|ToString(Integer) (Utilities|Array|Length _output_get)) "valid spawn points in the world."))
  ;[1 1 1] Spawn Required Items
  (for _array_element (Variables|Default|GetRequired%20Items)
    (bind _spawn_location (CallFunction|PopRandomSpawnLocation))
    (Game|SpawnActorfromClass _array_element (Transformation|GetWorldTransform (.arrow _spawn_location)) "AdjustIfPossibleButAlwaysSpawn" 0 0))
  ;[1 1 1] Spawn Optional Items
  (for _array_element_2 (Variables|Default|GetAvailable%20Spawn%20Points)
    (if (Math|Random|RandomBoolwithWeight (Variables|Default|GetChance%20To%20Spawn%20Optional%20Item))
      (bind _item (CallFunction|GetRandomOptionalItem))
      (Game|SpawnActorfromClass _item (Transformation|GetWorldTransform (.Arrow (Utilities|Struct|BreakS_ItemSpawnPoint _array_element_2))) "AdjustIfPossibleButAlwaysSpawn" 0 0))))

(event Collision|EventActorBeginOverlap
  (params (OtherActor :type Actor%20Object%20Reference)))

(event EventTick
  (params (DeltaSeconds :type Float%20%28single-precision%29)))

(fn ConstructionScript)

(fn PopRandomSpawnLocation
  (bind _available_spawn_points (Variables|Default|GetAvailable%20Spawn%20Points))
  (bind _returnvalue (Utilities|Array|Length _available_spawn_points))
  (bind _returnvalue_2 (- _returnvalue 1))
  (bind _item (Utilities|Array|Get(acopy) _available_spawn_points _returnvalue_2))
  (Utilities|Array|RemoveItem _available_spawn_points _item)
  (return _item))

(fn GetRandomOptionalItem
  (bind _optional_items (Variables|Default|GetOptional%20Items))
  (return (Utilities|Array|Get(acopy) _optional_items (- (Utilities|Array|Length _optional_items) 1))))