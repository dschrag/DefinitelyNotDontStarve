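; Parent Blueprint for cave segments in cave generation, with an empty OnCaveSpawned hook meant for the segment to place itself.
; RotateSelfToMatchDoors turns the actor in 90-degree yaw steps, rotating its door direction list clockwise until it matches the required world directions, and prints an error if none fit.
; GrabItemArrows, run from the construction script and CountItemSpawns, registers Arrow components tagged "item" as item spawn points.
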(event Custom|Count%20Item%20Spawns
  (CallFunction|GrabItemArrows))

(event Custom|On%20Cave%20Spawned)

(event EventBeginPlay)

(event Collision|EventActorBeginOverlap
  (params (OtherActor :type Actor%20Object%20Reference)))

(event EventTick
  (params (DeltaSeconds :type Float%20%28single-precision%29)))

(fn ConstructionScript
  (CallFunction|GrabItemArrows))

(fn RotateSelftoMatchDoors
  (params (Relative%20Door%20Directions :type Array%20of%20Enum_Directions%20Enums) (World%20Door%20Directions :type Array%20of%20Enum_Directions%20Enums))
  (LocalVariables|SetLocal%20World%20Door%20Directions World%20Door%20Directions)
  (bind _match (CallFunction|DirectionArraysMatch Relative%20Door%20Directions World%20Door%20Directions))
  (if _match
    (return)
    (else
      (LocalVariables|SetNew%20Relative%20Doors Relative%20Door%20Directions)
      (for _index (range 0 3)
        (Development|PrintString "Start Loop" false false)
        (Class|Actor|AddActorWorldRotation "0,90.000000, 0")
        (bind _out (CallFunction|RotateDirectionArray (LocalVariables|GetNew%20Relative%20Doors)))
        (LocalVariables|SetNew%20Relative%20Doors _out)
        (bind _match_2 (CallFunction|DirectionArraysMatch (LocalVariables|GetNew%20Relative%20Doors) (LocalVariables|GetLocal%20World%20Door%20Directions)))
        (if _match_2
          (Variables|Default|SetRelative%20Door%20Directions (LocalVariables|GetNew%20Relative%20Doors))
          (return)))
      ;[1 0.5048 0.01547] This is an error. Handle this better
      (Development|PrintString "The Cave Segment can't fit the requirements for this location." true true "(R=1.000000,G=0.008232,B=0.000000,A=1.000000)" 5.0)
      (return))))

(fn RotateDirectionClockwise
  (params (Input :type Enum_Directions%20Enum))
  (switch Utilities|FlowControl|Switch|SwitchonEnum_Directions Input
    (:NewEnumerator0
      (LocalVariables|SetTo%20Return "NewEnumerator2"))
    (:NewEnumerator1
      (LocalVariables|SetTo%20Return "NewEnumerator3"))
    (:NewEnumerator2
      (LocalVariables|SetTo%20Return "NewEnumerator1"))
    (:NewEnumerator3
      (LocalVariables|SetTo%20Return "NewEnumerator0")))
  (return (LocalVariables|GetTo%20Return)))

(fn DirectionArraysMatch
  (params (One :type Array%20of%20Enum_Directions%20Enums) (Two :type Array%20of%20Enum_Directions%20Enums))
  (if (== (Utilities|Array|Length One) (Utilities|Array|Length Two))
    (bind _array_element (Utilities|Array|ForEachLoopwithBreak One :!label _label)
      (:LoopBody
        (if (not (Utilities|Array|ContainsItem Two _array_element))
          (LocalVariables|SetDoMatch false)
          (goto _label Break)))
      (:Completed
        (return (LocalVariables|GetDoMatch))))
    (else
      (return false))))

(fn RotateDirectionArray
  (params (In :type Array%20of%20Enum_Directions%20Enums))
  (for _array_element In
    (bind _output (CallFunction|RotateDirectionClockwise _array_element))
    (Utilities|Array|Add (LocalVariables|GetTo%20Return) _output)
    (Development|PrintString (Utilities|String|EnumtoString _output) false false "(R=0.000000,G=0.660000,B=1.000000,A=1.000000)" 1e+01))
  (return (LocalVariables|GetTo%20Return)))

(fn GrabItemArrows
  (for _array_element (Actor|GetComponentsbyTag "/Script/Engine.ArrowComponent" "item")
    (Utilities|Array|AddUnique (Variables|Default|GetItem%20Spawn%20Points) (Utilities|Struct|MakeS_ItemSpawnPoint _array_element self)))
  (Development|PrintString (Utilities|String|Append "There are this many spawns on this cave: " (Utilities|String|ToString(Integer) (Utilities|Array|Length (Variables|Default|GetItem%20Spawn%20Points)))) false true "(R=1.000000,G=0.138182,B=0.777511,A=1.000000)" 1e+01)
  (return))