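; BP_BasicXCave_Pillar is a cave section actor for cave generation, an X-shaped piece with a pillar.
; On BeginPlay it rotates the whole actor by a random multiple of 90 degrees in yaw, varying its orientation while staying grid-aligned.
; It then gives the Pillar and StaticMesh9 components independent random world yaw so repeated sections look different.
; The construction script is empty.
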(event EventBeginPlay
  (Utilities|RandomizeRotation)
  (Transformation|SetWorldRotation (Variables|Default|GetPillar) (Math|Rotator|MakeRotator 0.0 0.0 (Math|Random|RandomFloatinRange 0.0 3.6e+02)) false false)
  (Transformation|SetWorldRotation (Variables|Default|GetStaticMesh9) (Math|Rotator|MakeRotator 0.0 0.0 (Math|Random|RandomFloatinRange 0.0 3.6e+02)) false false))

(event Collision|EventActorBeginOverlap
  (params (OtherActor :type Actor%20Object%20Reference)))

(event EventTick
  (params (DeltaSeconds :type Float%20%28single-precision%29)))

(fn ConstructionScript)