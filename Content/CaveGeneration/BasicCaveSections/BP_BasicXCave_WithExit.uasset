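; BP_BasicXCave_WithExit is a cave section for procedural cave generation that carries the level exit ladder.
; On OnCaveSpawned it turns itself by a random multiple of 90 degrees, gives one static mesh a random world yaw, then calls GrabItemArrows.
; On BeginPlay it spawns BP_CaveLevelLadder at its Arrow component's transform, facing along that arrow.
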(event Collision|EventActorBeginOverlap
  (params (OtherActor :type Actor%20Object%20Reference)))

(event EventTick
  (params (DeltaSeconds :type Float%20%28single-precision%29)))

(event EventOnCaveSpawned
  (Utilities|RandomizeRotation)
  (Transformation|SetWorldRotation (Variables|Default|GetStaticMesh9) (Math|Rotator|MakeRotator 0.0 0.0 (Math|Random|RandomFloatinRange 0.0 3.6e+02)) false false)
  (CallFunction|GrabItemArrows))

(event EventBeginPlay
  (bind _arrow (Variables|Default|GetArrow))
  (bind _returnvalue (Transformation|GetWorldTransform _arrow))
  (Game|SpawnActorfromClass "/Game/CaveGeneration/BP_CaveLevelLadder.BP_CaveLevelLadder_C" (Math|Transform|MakeTransform (.location _returnvalue) (Math|Conversions|RotationFromXVector (Math|Vector|GetForwardVector _arrow)) (.scale _returnvalue)) "Undefined" 0 0))

(fn ConstructionScript)