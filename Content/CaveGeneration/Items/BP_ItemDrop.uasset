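; Crate item drop for the cave generation content, with staged visual damage.
; On BeginPlay it spawns an ItemBP actor at the Arrow component's transform.
; Each OnPartiallyDestroy event decrements Health and swaps the Crate mesh between intact, damaged and destroyed open-crate variants.
; The actor and its spawned item are not removed when the crate reaches the destroyed state.
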(event Custom|On%20Partially%20Destroy
  (bind _crate (Variables|Default|GetCrate))
  (bind _result (Math|Integer|DecrementInt (Variables|Default|GetHealth))
    (:%20%20
      (bind _output_get (Variables|Default|SetHealth _result))
      (switch int _output_get
        (:Default
          (Components|StaticMesh|SetStaticMesh _crate "/Game/InfinityBladeGrassLands/Environments/Misc/Exo_Deco01/StaticMesh/SM_Exo_Crate_Open_Destroyed.SM_Exo_Crate_Open_Destroyed" :!label _label))
        (:0
          (goto _label))
        (:1
          (Components|StaticMesh|SetStaticMesh _crate "/Game/InfinityBladeGrassLands/Environments/Misc/Exo_Deco01/StaticMesh/SM_Exo_Crate_Open_Damaged.SM_Exo_Crate_Open_Damaged"))
        (:2
          (Components|StaticMesh|SetStaticMesh _crate "/Game/InfinityBladeGrassLands/Environments/Misc/Exo_Deco01/StaticMesh/SM_Exo_Crate_Open_Intact.SM_Exo_Crate_Open_Intact"))))))

(event EventBeginPlay
  (Game|SpawnActorfromClass (Variables|Default|GetItemBP) (Transformation|GetWorldTransform (Variables|Default|GetArrow)) "Undefined" 0 0))

(event Collision|EventActorBeginOverlap
  (params (OtherActor :type Actor%20Object%20Reference)))

(event EventTick
  (params (DeltaSeconds :type Float%20%28single-precision%29)))

(fn ConstructionScript)