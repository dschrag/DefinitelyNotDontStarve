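; BP_InventoryArea is an inventory area that displays added items as physical piles in the world.
; OnAddItem casts the new item to stones, bread or rat carcass and sends it to the matching pile point, ignoring other types.
; Spawn in Pile line-traces within a narrow random cone built from a forward vector, then teleports the existing item to the hit location with random rotation.
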(event Custom|On%20Add%20Item
  (params (New%20Item :type BP%20Item%20Parent%20Object%20Reference))
  (bind _asbp_stones_item (Utilities|Casting|CastToBP_StonesItem New%20Item)
    (:then
      (Utilities|SpawninPile (Variables|Default|GetRock%20Pile) _asbp_stones_item))
    (:CastFailed
      (bind _asbp_bread (Utilities|Casting|CastToBP_Bread New%20Item)
        (:then
          (Utilities|SpawninPile (Variables|Default|GetBread%20Spawn) _asbp_bread))
        (:CastFailed
          (bind _asbp_rat_carcas (Utilities|Casting|CastToBP_RatCarcas New%20Item))
          (Utilities|SpawninPile (Variables|Default|GetRat%20Bodies) _asbp_rat_carcas))))))

(event EventBeginPlay)

(event Collision|EventActorBeginOverlap
  (params (OtherActor :type Actor%20Object%20Reference)))

(event EventTick
  (params (DeltaSeconds :type Float%20%28single-precision%29)))

(fn ConstructionScript)